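; BP_URSocket is a socket client actor that links the game to a server on the local machine.
; It connects on BeginPlay and stores the connection ID, which SendState uses to send outgoing data.
; Incoming messages have their first element converted to a BP_URPacket type, then the Receive dispatcher broadcasts that packet with the remaining data.
; Connection and disconnection callbacks are empty, and the Disconnect call never runs.
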(event Custom|Disconnected
  (params (ConnectionId :type Integer)))

(event Custom|Connected
  (params (ConnectionId :type Integer)))

(event Custom|ReceiveMessage
  (params (ConnectionId :type Integer) (Message :type Array%20of%20Bytes))
  (Variables|Default|SetURPacket (Utilities|Enum|ByteToEnumBP_URPacket (Utilities|Array|Get(acopy) Message)))
  (Utilities|Array|RemoveIndex Message)
  (Default|CallReceive (Variables|Default|GetURPacket) Message))

(event Custom|SendState
  (params (DataToSend :type Array%20of%20Bytes))
  (Class|TcpSocketConnection|SendData (Variables|Default|GetId) DataToSend))

(event EventBeginPlay
  (bind _connectionid (Class|TcpSocketConnection|Connect "127.0.0.1" 9999 (delegate Custom|Disconnected) (delegate Custom|Connected) (delegate Custom|ReceiveMessage)))
  (Variables|Default|SetId _connectionid))

(event Collision|EventActorBeginOverlap
  (params (OtherActor :type Actor%20Object%20Reference)))

(event EventTick
  (params (DeltaSeconds :type Float%20%28single-precision%29)))

(fn ConstructionScript)